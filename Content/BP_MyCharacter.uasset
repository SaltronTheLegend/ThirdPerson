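; Player character Blueprint with a cooldown-gated dash and a scripted gun pickup that opens an exit door.
; Dash uses a timeline to move the actor unswept along the last movement input, with camera shake.
; Zoom and Reverse events animate spring arm length through timelines.
; Pressing E, when allowed, attaches a gun to the mesh socket, restores walking, calls Reverse, triggers BP_D's Door component and plays sounds.
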(event `InputAction|Dash`
  (params (Key :type "Key Structure"))
  (bind _returnvalue (`self.K2_GetActorLocation`))
  (:`Pressed`
    (if (`self.bCanDash `)
      (bind (_direction _newtrack_0) (`Timeline|Dash Timeline`)
        (:`Update`
          (`self.K2_SetActorLocation` (`KismetMathLibrary.VLerp` _returnvalue (+ _returnvalue (* (`self.Dash Distance`) (`KismetMathLibrary.Normal` (`self.GetLastMovementInputVector`)))) _newtrack_0))
          (`GameplayStatics.PlayWorldCameraShake` null)
          (set `self.bCanDash ` false)
          (`KismetSystemLibrary.Delay` (`self.DashCooldown `))
          (set `self.bCanDash ` true))))))

(event `Reverse`
  (bind (_direction _camera_fov _armlengthtrack) (`Timeline|UnZoomTimeline`)
    (:`Update`
      (set `SpringArmComponent.TargetArmLength` _armlengthtrack (`self.SpringArm`)))))

(event `Zoom`
  (bind (_direction _camera_fov _armlengthtrack) (`Timeline|ZoomTimeline`)
    (:`Update`
      (set `SpringArmComponent.TargetArmLength` _armlengthtrack (`self.SpringArm`)))))

(event `Key|E`
  (params (Key :type "Key Structure"))
  (:`Pressed`
    (if (`self.CanTakeGun`)
      (bind _returnvalue (`AddComponent|NODE_AddChildActorComponent-1`))
      (`self.K2_AttachToComponent` (`ChildActorComponent.ChildActor` _returnvalue) (`self.Mesh`) "GunSocket" "SnapToTarget" "SnapToTarget" "SnapToTarget" true)
      (set `self.GunTaken` true)
      (`CharacterMovementComponent.SetMovementMode` (`self.CharacterMovement`) "MOVE_Walking" 0)
      (`self.Reverse`)
      (`GameplayStatics.PlaySound2D` "/Game/Sounds/UwillPay.UwillPay" 1.0 1.0 0.0 null null)
      (bind _outactors (`GameplayStatics.GetAllActorsOfClass` "/Game/BP_D.BP_D_C"))
      (`Door.TriggerExitDoorOpen` (`self.GetComponentByClass` (`|GetArrayItem` _outactors) "/Script/ThirdPerson.Door"))
      (`KismetSystemLibrary.Delay` 5.0)
      (`GameplayStatics.PlaySound2D` "/Game/Sounds/ExitSound.ExitSound" 1.0 1.0 0.0 null null))))

(fn `UserConstructionScript`)